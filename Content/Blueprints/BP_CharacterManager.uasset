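; Character manager for a random BP_SmashCharacter picker, holding the full, filtered and selected rosters.
; On BeginPlay it gathers the character actors, insertion-sorts them by SortNumber and applies index-matched weights and enabled flags from BP_SaveManager.
; It filters to enabled characters, then draws without replacement, either uniformly or with odds proportional to 1/Weight.
; Incrementing a selected character's Weight lowers its future weighted odds and triggers a save.
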(event `self.ReceiveBeginPlay`
  (bind _smashcharsarray (`self.Create All Character Array`))
  (set `self.AllCharacterArray` _smashcharsarray))

(fn `Create All Character Array`
  (returns (SmashCharsArray :type "Array of /Game/Blueprints/SmashCharacters/BP_SmashCharacter Object Reference"))
  (locals (SortedArray :type "Array of /Game/Blueprints/SmashCharacters/BP_SmashCharacter Object Reference"))
  (bind _outactors (`GameplayStatics.GetAllActorsOfClass` "/Game/Blueprints/SmashCharacters/BP_SmashCharacter.BP_SmashCharacter_C"))
  (for _array_element _outactors
    (`KismetSystemLibrary.PrintString` (`KismetStringLibrary.Concat_StrStr` "Found BP_SmashCharacter: " (`/Game/Blueprints/SmashCharacters/BP_SmashCharacter.Name` _array_element))))
  (bind _sorted_array (`self.Sort Array` _outactors))
  (set `local.SortedArray` _sorted_array)
  (bind _returnvalue (`GameplayStatics.GetActorOfClass` "/Game/Blueprints/BP_SaveManager.BP_SaveManager_C"))
  (bind _savegame (`/Game/Blueprints/BP_SaveManager.Load Game` _returnvalue))
  (`/Engine/EditorBlueprintResources/StandardMacros.IsValid` _savegame
    (:`Is Valid`
      (for (_array_element_2 _array_index) (`local.SortedArray`)
        (set `/Game/Blueprints/SmashCharacters/BP_SmashCharacter.Weight` (`|GetArrayItem` (`/Game/Blueprints/MySaveGame.CharacterWeights` _savegame) _array_index) _array_element_2)
        (set `/Game/Blueprints/SmashCharacters/BP_SmashCharacter.Enabled` (`|GetArrayItem` (`/Game/Blueprints/MySaveGame.CharactersEnabled` _savegame) _array_index) _array_element_2)))
    (:`Is Not Valid`
      _))
  (return (`local.SortedArray`)))

(fn `Create Filtered Character Array`
  (locals (`Local Array` :type "Array of /Game/Blueprints/SmashCharacters/BP_SmashCharacter Object Reference"))
  (for _array_element (`self.AllCharacterArray`)
    (if (`/Game/Blueprints/SmashCharacters/BP_SmashCharacter.Enabled` _array_element)
      (`KismetArrayLibrary.Array_Add` (`local.Local Array`) _array_element)))
  (`KismetSystemLibrary.PrintString` "Array complete")
  (set `self.FilteredCharacterArray` (`local.Local Array`)))

(fn `Create Split Character Arrays`
  (returns (StandardCharacterArray :type "Array of /Game/Blueprints/SmashCharacters/BP_SmashCharacter Object Reference") (NonStandardCharacterArray :type "Array of /Game/Blueprints/SmashCharacters/BP_SmashCharacter Object Reference"))
  (locals (LocalStandardCharacterArray :type "Array of /Game/Blueprints/SmashCharacters/BP_SmashCharacter Object Reference") (LocalNonStandardCharacterArray :type "Array of /Game/Blueprints/SmashCharacters/BP_SmashCharacter Object Reference"))
  (for _array_element (`self.AllCharacterArray`)
    (if (`/Game/Blueprints/SmashCharacters/BP_SmashCharacter.StandardCharacter` _array_element)
      (`KismetArrayLibrary.Array_Add` (`local.LocalStandardCharacterArray`) _array_element)
      (else
        (`KismetArrayLibrary.Array_Add` (`local.LocalNonStandardCharacterArray`) _array_element))))
  (return (`local.LocalStandardCharacterArray`) (`local.LocalNonStandardCharacterArray`)))

(fn `Get Sum of Filtered Character Weights`
  (set `self.TotalWeight` 0.0)
  (for _array_element (`self.FilteredCharacterArray`)
    (set `self.TotalWeight` (+ (`self.TotalWeight`) (`KismetMathLibrary.SafeDivide` 1.0 (`KismetMathLibrary.Conv_IntToDouble` (`/Game/Blueprints/SmashCharacters/BP_SmashCharacter.Weight` _array_element))))))
  (`KismetSystemLibrary.PrintString` (`KismetStringLibrary.Concat_StrStr` "Total Weight Set To " (`KismetStringLibrary.Conv_DoubleToString` (`self.TotalWeight`)))))

(fn `Increase Weight of Selected Character`
  (params (`Character Index` :type Integer))
  (bind _output (`|GetArrayItem` (`self.SelectedCharacterArray`) `Character Index`))
  (bind _result (`/Engine/EditorBlueprintResources/StandardMacros.IncrementInt` (`/Game/Blueprints/SmashCharacters/BP_SmashCharacter.Weight` _output))
    (:`  `
      (bind _output_get (set `/Game/Blueprints/SmashCharacters/BP_SmashCharacter.Weight` _result _output))
      (`KismetSystemLibrary.PrintString` (`KismetStringLibrary.Concat_StrStr` "Character Weight Set To: " (`KismetStringLibrary.Conv_IntToString` _output_get)))
      (bind _returnvalue (`GameplayStatics.GetActorOfClass` "/Game/Blueprints/BP_SaveManager.BP_SaveManager_C"))
      (bind _savegame (`/Game/Blueprints/BP_SaveManager.Load Game` _returnvalue))
      (`/Game/Blueprints/BP_SaveManager.Save Game` _returnvalue (`/Game/Blueprints/MySaveGame.Instant Random` _savegame)))))

(fn `Select Random Characters NonWeighted`
  (params (Amount :type Integer))
  (locals (`Local Array` :type "Array of /Game/Blueprints/SmashCharacters/BP_SmashCharacter Object Reference") (CurrentCharacter :type "/Game/Blueprints/SmashCharacters/BP_SmashCharacter Object Reference"))
  (bind _filteredcharacterarray (`self.FilteredCharacterArray`))
  (for _ (range 1 (+ Amount 1))
    (bind _output_get (set `local.CurrentCharacter` (`|GetArrayItem` _filteredcharacterarray (`KismetMathLibrary.RandomInteger` (`KismetArrayLibrary.Array_Length` _filteredcharacterarray)))))
    (`KismetArrayLibrary.Array_Add` (`local.Local Array`) _output_get)
    (`KismetArrayLibrary.Array_RemoveItem` (`self.FilteredCharacterArray`) _output_get))
  (set `self.SelectedCharacterArray` (`local.Local Array`)))

(fn `Select Random Characters Weighted`
  (params (Amount :type Integer))
  (locals (CurrentWeight :type "Float (double-precision)") (SelectedFloat :type "Float (double-precision)") (LocalArray :type "Array of /Game/Blueprints/SmashCharacters/BP_SmashCharacter Object Reference"))
  (bind _totalweight (`self.TotalWeight`))
  (for _ (range 1 (+ Amount 1))
    (bind _output_get (set `local.SelectedFloat` (`KismetMathLibrary.RandomFloatInRange` 0.0 _totalweight)))
    (`KismetSystemLibrary.PrintString` (`KismetStringLibrary.Concat_StrStr` "Selected Float Value: " (`KismetStringLibrary.Conv_DoubleToString` _output_get) "Maximum Float Value: " (`KismetStringLibrary.Conv_DoubleToString` _totalweight)) true true (struct :`R` 0.073356 :`G` 0.463542 :`A` 1.0) 15.0)
    (for _array_element (`self.FilteredCharacterArray`)
      (bind _returnvalue (`KismetMathLibrary.SafeDivide` 1.0 (`KismetMathLibrary.Conv_IntToDouble` (`/Game/Blueprints/SmashCharacters/BP_SmashCharacter.Weight` _array_element))))
      (bind _output_get_2 (set `local.CurrentWeight` (+ (`local.CurrentWeight`) _returnvalue)))
      (if (>= _output_get_2 (`local.SelectedFloat`))
        (`KismetArrayLibrary.Array_Add` (`local.LocalArray`) _array_element)
        (set `local.CurrentWeight` 0.0)
        (bind _output_get_3 (set `self.TotalWeight` (- (`self.TotalWeight`) _returnvalue)))
        (`KismetArrayLibrary.Array_RemoveItem` (`self.FilteredCharacterArray`) _array_element)
        (`KismetSystemLibrary.PrintString` (`KismetStringLibrary.Conv_DoubleToString` _output_get_3) true true (struct :`R` 0.453125 :`B` 0.011852 :`A` 1.0))
        (break))))
  (bind _output_get_4 (set `self.SelectedCharacterArray` (`local.LocalArray`)))
  (for _array_element_2 _output_get_4
    (`KismetSystemLibrary.PrintString` (`/Game/Blueprints/SmashCharacters/BP_SmashCharacter.Name` _array_element_2))))

(fn `Sort Array`
  (params (TargetArray :type "Array of /Game/Blueprints/SmashCharacters/BP_SmashCharacter Object Reference (by ref)"))
  (returns (`Sorted Array` :type "Array of /Game/Blueprints/SmashCharacters/BP_SmashCharacter Object Reference"))
  (locals (`Sorting List` :type "Array of /Game/Blueprints/SmashCharacters/BP_SmashCharacter Object Reference") (`Current Target` :type "/Game/Blueprints/SmashCharacters/BP_SmashCharacter Object Reference") (`Current Target Stepper` :type Integer) (ShouldSearch :type Boolean :default true))
  (bind _sorting_list (`local.Sorting List`))
  (bind _output (`|GetArrayItem` (`local.Sorting List`) (- (`local.Current Target Stepper`) 1)))
  (for (_array_element _array_index) TargetArray
    (set `local.Current Target` _array_element)
    (set `local.Current Target Stepper` _array_index)
    (set `local.ShouldSearch` true)
    (while (`local.ShouldSearch`)
      (`/Engine/EditorBlueprintResources/StandardMacros.IsValid` _output
        (:`Is Valid`
          (if (> (`/Game/Blueprints/SmashCharacters/BP_SmashCharacter.SortNumber` _output) (`/Game/Blueprints/SmashCharacters/BP_SmashCharacter.SortNumber` (`local.Current Target`)))
            (set `local.Current Target Stepper` (- (`local.Current Target Stepper`) 1))
            (else
              (set `local.ShouldSearch` false))))
        (:`Is Not Valid`
          (set `local.ShouldSearch` false))))
    (`KismetArrayLibrary.Array_Insert` _sorting_list (`local.Current Target`) (`local.Current Target Stepper`))
    (for _array_element_2 _sorting_list
      (`KismetSystemLibrary.PrintString` (`KismetStringLibrary.Conv_IntToString` (`/Game/Blueprints/SmashCharacters/BP_SmashCharacter.SortNumber` _array_element_2)))))
  (return (`local.Sorting List`)))

(fn `UserConstructionScript`)