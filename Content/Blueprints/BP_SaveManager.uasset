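; BP_SaveManager is an actor that saves and loads character weights and an InstantRandom value through a MySaveGame object.
; Save Game creates a fresh save object, copies each Weight from BP_CharacterManager's AllCharacterArray, stores the passed InstantRandom, and writes to a single fixed slot.
; Load Game reads that slot and returns the cast MySaveGame, leaving callers to apply the data.
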(fn `Load Game`
  (returns (SaveGame :type "/Game/Blueprints/MySaveGame Object Reference"))
  (bind _returnvalue (`GameplayStatics.LoadGameFromSlot` "SaveSlot"))
  (bind _asmy_save_game (cast `/Game/Blueprints/MySaveGame` _returnvalue))
  (return _asmy_save_game))

(fn `Save Game`
  (params (`Instant Random` :type Boolean))
  (locals (SaveGame :type "/Game/Blueprints/MySaveGame Object Reference"))
  (bind _savegame (`local.SaveGame`))
  (bind _returnvalue (`GameplayStatics.CreateSaveGameObject` "/Game/Blueprints/MySaveGame.MySaveGame_C"))
  (bind _output_get (set `local.SaveGame` _returnvalue))
  (bind _returnvalue_2 (`GameplayStatics.GetActorOfClass` "/Game/Blueprints/BP_CharacterManager.BP_CharacterManager_C"))
  (for _array_element (`/Game/Blueprints/BP_CharacterManager.AllCharacterArray` _returnvalue_2)
    (`KismetArrayLibrary.Array_Add` (`/Game/Blueprints/MySaveGame.CharacterWeights` _output_get) (`/Game/Blueprints/SmashCharacters/BP_SmashCharacter.Weight` _array_element)))
  (set `/Game/Blueprints/MySaveGame.Instant Random` (`local.Instant Random`) _savegame)
  (`GameplayStatics.SaveGameToSlot` _savegame "SaveSlot"))

(fn `UserConstructionScript`)