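; Actor Blueprint that holds a Smash Bros. character roster and randomly picks characters, favoring those with lower Weight.
; BeginPlay builds the roster, and separate functions filter out zero-weight entries and total the inverse weights.
; Selection draws without replacement by walking cumulative 1/Weight against a random float, shrinking the pool and total after each pick.
; Another function raises a selected character's Weight in the roster, lowering its odds in later draws.
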(event `self.ReceiveBeginPlay`
  (bind _array (`self.Create All Character Array`))
  (set `self.AllCharacterArray` _array))

(fn `Create All Character Array`
  (returns (Array :type "Array of /Game/SmashCharacterStruct Structure"))
  (return (`|MakeArray` (`self.MarioCharacter`) (`self.DonkeyKongCharacter`) (`self.LinkCharacter`) (`self.PikachuCharacter`) (`self.KirbyCharacter`) (`self.SamusCharacter`))))

(fn `Create Filtered Character Array`
  (set `self.FilteredCharacterArray` (`|MakeArray` (struct) :!type "/Game/SmashCharacterStruct Structure"))
  (for _array_element (`self.AllCharacterArray`)
    (if (not (== (`.Weight_8_8EE5C2334A489517AEA0BB94B745D178` (break `/Game/SmashCharacterStruct` _array_element)) 0))
      (`KismetArrayLibrary.Array_Add` (`self.FilteredCharacterArray`) _array_element)))
  (`KismetSystemLibrary.PrintString` "Array complete"))

(fn `Get Sum of Filtered Character Weights`
  (set `self.TotalWeight` 0.0)
  (for _array_element (`self.FilteredCharacterArray`)
    (set `self.TotalWeight` (+ (`self.TotalWeight`) (`KismetMathLibrary.SafeDivide` 1.0 (`KismetMathLibrary.Conv_IntToDouble` (`.Weight_8_8EE5C2334A489517AEA0BB94B745D178` (break `/Game/SmashCharacterStruct` _array_element)))))))
  (`KismetSystemLibrary.PrintString` (`KismetStringLibrary.Concat_StrStr` "Total Weight Set To " (`KismetStringLibrary.Conv_DoubleToString` (`self.TotalWeight`)))))

(fn `Increase Weight of Selected Character`
  (params (`Character Index` :type Integer))
  (bind _output (`|GetArrayItem` (`self.SelectedCharacterArray`) `Character Index`))
  (bind _returnvalue (`KismetArrayLibrary.Array_Find` (`self.AllCharacterArray`) _output))
  (bind _result (`/Engine/EditorBlueprintResources/StandardMacros.IncrementInt` (`.Weight_8_8EE5C2334A489517AEA0BB94B745D178` (break `/Game/SmashCharacterStruct` _output)))
    (:`  `
      (if (>= _returnvalue 0)
        (setmembers `/Game/SmashCharacterStruct` :`StructRef` (`|GetArrayItem` (`self.AllCharacterArray`) _returnvalue) :`Weight` _result)
        (`KismetSystemLibrary.PrintString` (`KismetStringLibrary.Concat_StrStr` "Character Weight Set To: " (`KismetStringLibrary.Conv_IntToString` _result)))
        (else
          (`KismetSystemLibrary.PrintString` "Could not find in All Char Array" true true (struct :`R` 1.0 :`A` 1.0) 10.0))))))

(fn `Select Random Characters`
  (params (Amount :type Integer))
  (locals (CurrentWeight :type "Float (double-precision)") (SelectedFloat :type "Float (double-precision)") (LocalArray :type "Array of /Game/SmashCharacterStruct Structure"))
  (bind _totalweight (`self.TotalWeight`))
  (for _ (range 1 (+ Amount 1))
    (bind _output_get (set `local.SelectedFloat` (`KismetMathLibrary.RandomFloatInRange` 0.0 _totalweight)))
    (`KismetSystemLibrary.PrintString` (`KismetStringLibrary.Concat_StrStr` "Selected Float Value: " (`KismetStringLibrary.Conv_DoubleToString` _output_get) "Maximum Float Value: " (`KismetStringLibrary.Conv_DoubleToString` _totalweight)) true true (struct :`R` 0.073356 :`G` 0.463542 :`A` 1.0) 15.0)
    (for _array_element (`self.FilteredCharacterArray`)
      (bind _returnvalue (`KismetMathLibrary.SafeDivide` 1.0 (`KismetMathLibrary.Conv_IntToDouble` (`.Weight_8_8EE5C2334A489517AEA0BB94B745D178` (break `/Game/SmashCharacterStruct` _array_element)))))
      (bind _output_get_2 (set `local.CurrentWeight` (+ (`local.CurrentWeight`) _returnvalue)))
      (if (>= _output_get_2 (`local.SelectedFloat`))
        (`KismetArrayLibrary.Array_Add` (`local.LocalArray`) _array_element)
        (set `local.CurrentWeight` 0.0)
        (bind _output_get_3 (set `self.TotalWeight` (- (`self.TotalWeight`) _returnvalue)))
        (`KismetArrayLibrary.Array_RemoveItem` (`self.FilteredCharacterArray`) _array_element)
        (`KismetSystemLibrary.PrintString` (`KismetStringLibrary.Conv_DoubleToString` _output_get_3) true true (struct :`R` 0.453125 :`B` 0.011852 :`A` 1.0))
        (break))))
  (bind _output_get_4 (set `self.SelectedCharacterArray` (`local.LocalArray`)))
  (for _array_element_2 _output_get_4
    (`KismetSystemLibrary.PrintString` (`.Name_5_FF84FF1B401B7941CDBD08B05F47E885` (break `/Game/SmashCharacterStruct` _array_element_2)))))

(fn `UserConstructionScript`)